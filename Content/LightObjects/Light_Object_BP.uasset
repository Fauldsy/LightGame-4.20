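; Light-reactive object that fades its material through a timeline when the combined colour of the lights reaching it matches its own colour.
; Each Tick it checks the GameMode's directional, point and spot lights, testing attenuation radius and, for spots, cone angle.
; Light colours combine additively as RGB flags into one colour, which sets Lit and plays or reverses the fade.
; Pressing N prints the light count for debugging.
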(event `Key|N`
  (params (Key :type "Key Structure"))
  (:`Pressed`
    (`KismetSystemLibrary.PrintString` (`KismetStringLibrary.Concat_StrStr` "Number of lights: " (`KismetStringLibrary.Conv_IntToString` (`self.NumberOfLights`))))))

(event `self.ReceiveBeginPlay`
  (bind _asfirst_person_game_mode (cast `/Game/FirstPersonBP/Blueprints/FirstPersonGameMode` (`GameplayStatics.GetGameMode`)))
  (set `self.GameMode` _asfirst_person_game_mode)
  (`self.EnableInput` (`GameplayStatics.GetPlayerController` 0))
  (bind _returnvalue (`PrimitiveComponent.CreateDynamicMaterialInstance` (`self.Cube`) 0 "/Game/Shaders/MAT_AlphaBlend_Inst.MAT_AlphaBlend_Inst"))
  (set `self.FadeObject` _returnvalue)
  (`self.IsLightRed`))

(event `self.ReceiveTick`
  (params (DeltaSeconds :type "Float (single-precision)"))
  (`self.CheckOverlap`)
  (if (`self.Lit`)
    (bind (_direction _floattrack) (`Timeline|FadeIn` :!label _label)
      (:`Update`
        (`MaterialInstanceDynamic.SetScalarParameterValue` (`self.FadeObject`) "Fade" _floattrack)))
    (else
      (goto _label :!via `Reverse`))))

(fn `AngleBetweenVectors`
  (params (Vector1 :type "Vector Structure") (Vector2 :type "Vector Structure"))
  (returns (Angle :type "Float (double-precision)"))
  (return (`KismetMathLibrary.DegAcos` (`KismetMathLibrary.Dot_VectorVector` (`KismetMathLibrary.Normal` Vector1) (`KismetMathLibrary.Normal` Vector2)))))

(fn `CheckDirectionalLights`
  (params (DirectionalLights :type "Array of /Game/Lights/Directional/DirectionalLightSource_BP Object Reference"))
  (for _array_element DirectionalLights
    (`self.ToggleRGBLit` (`/Game/Lights/BaseLightSource_BP.Colour_ENUM` _array_element)))
  (return))

(fn `CheckOverlap`
  (returns (IsLit :type Boolean))
  (bind _gamemode (`self.GameMode`))
  (`self.ClearLit`)
  (`self.CheckDirectionalLights` (`/Game/FirstPersonBP/Blueprints/FirstPersonGameMode.DirectionalLights` _gamemode))
  (`self.CheckPointLights` (`/Game/FirstPersonBP/Blueprints/FirstPersonGameMode.PointLights` _gamemode))
  (`self.CheckSpotLights` (`/Game/FirstPersonBP/Blueprints/FirstPersonGameMode.SpotLights` _gamemode))
  (bind _islit (`self.IsLit`))
  (return _islit))

(fn `CheckPointLights`
  (params (PointLights :type "Array of /Game/Lights/Point_Spot/PointLightSource_BP Object Reference"))
  (for _array_element PointLights
    (bind _pointlight (`/Game/Lights/Point_Spot/PointLightSource_BP.PointLight` _array_element))
    (if (>= (`PointLightComponent.AttenuationRadius` _pointlight) (`KismetMathLibrary.VSize` (- (`SceneComponent.K2_GetComponentLocation` _pointlight) (`SceneComponent.K2_GetComponentLocation` (`self.Mesh`)))))
      (`self.ToggleRGBLit` (`/Game/Lights/BaseLightSource_BP.Colour_ENUM` _array_element))))
  (return))

(fn `CheckSpotLights`
  (params (SpotLights :type "Array of /Game/Lights/Point_Spot/SpotLightSource_BP Object Reference"))
  (for _array_element SpotLights
    (bind _testlight (`/Game/Lights/Point_Spot/SpotLightSource_BP.TestLight` _array_element))
    ;[1 1 1] Is in Attenuation Radius
    (if (>= (`PointLightComponent.AttenuationRadius` _testlight) (`KismetMathLibrary.VSize` (- (`SceneComponent.K2_GetComponentLocation` _testlight) (`SceneComponent.K2_GetComponentLocation` (`self.Mesh`)))))
      (bind _testlight_2 (`/Game/Lights/Point_Spot/SpotLightSource_BP.TestLight` _array_element))
      ;[1 1 1] To Do Check if in light cone
      (bind _angle (`self.AngleBetweenVectors` (- (`SceneComponent.K2_GetComponentLocation` (`self.Mesh`)) (`SceneComponent.K2_GetComponentLocation` _testlight_2)) (`SceneComponent.GetForwardVector` _testlight_2)))
      (if (<= _angle (`SpotLightComponent.OuterConeAngle` _testlight_2))
        (`self.ToggleRGBLit` (`/Game/Lights/BaseLightSource_BP.Colour_ENUM` _array_element)))))
  (return))

(fn `ClearLit`
  (set `self.RedLit` false)
  (set `self.GreenLit` false)
  (set `self.BlueLit` false))

(fn `CombinedLightColour`
  (returns (LightColour :type "/Game/Enums/Colours8_ENUM Enum"))
  (locals (ReturnedColour_LOCAL :type "/Game/Enums/Colours8_ENUM Enum"))
  (if (`self.RedLit`)
    (if (`self.GreenLit`)
      (if (`self.BlueLit`)
        (return "NewEnumerator6")
        (else
          (return "NewEnumerator3")))
      (elif (`self.BlueLit`)
        (return "NewEnumerator5")
        (else
          (return "NewEnumerator0"))))
    (elif (`self.GreenLit`)
      (if (`self.BlueLit`)
        (return "NewEnumerator4")
        (else
          (return "NewEnumerator1")))
      (elif (`self.BlueLit`)
        (return "NewEnumerator2")
        (else
          (return "NewEnumerator7"))))))

(fn `IsLightRed`
  (if (> (`self.NumberOfLights`) 0)
    (if (`|EnumEquality` (`/Game/Lights/BaseLightSource_BP.Colour_ENUM` (`|GetArrayItem` (`/Game/FirstPersonBP/Blueprints/FirstPersonGameMode.SpotLights` (`self.GameMode`)))) "NewEnumerator0")
      (set `self.Lit` true)
      (else
        (set `self.Lit` false)))
    (else
      (`KismetSystemLibrary.PrintString` "No Lights"))))

(fn `IsLit`
  (returns (IsLit :type Boolean))
  (bind _lightcolour (`self.CombinedLightColour`))
  (if (`|EnumEquality` (`self.ObjectColour`) _lightcolour)
    (set `self.Lit` true)
    (else
      (set `self.Lit` false)))
  (return (`self.Lit`)))

(fn `NumberOfLights`
  (returns (NumberOfLights :type Integer))
  (bind _gamemode (`self.GameMode`))
  (return (+ (`KismetArrayLibrary.Array_Length` (`/Game/FirstPersonBP/Blueprints/FirstPersonGameMode.SpotLights` _gamemode)) (`KismetArrayLibrary.Array_Length` (`/Game/FirstPersonBP/Blueprints/FirstPersonGameMode.DirectionalLights` _gamemode)) (`KismetArrayLibrary.Array_Length` (`/Game/FirstPersonBP/Blueprints/FirstPersonGameMode.PointLights` _gamemode)))))

(fn `ToggleRGBLit`
  (params (Light :type "/Game/Enums/Colours8_ENUM Enum" :default "NewEnumerator0"))
  (switch `/Game/Enums/Colours8_ENUM` Light
    (:`NewEnumerator0`
      (set `self.RedLit` true))
    (:`NewEnumerator3`
      (set `self.RedLit` true)
      (set `self.GreenLit` true))
    (:`NewEnumerator1`
      (set `self.GreenLit` true))
    (:`NewEnumerator4`
      (set `self.GreenLit` true)
      (set `self.BlueLit` true))
    (:`NewEnumerator2`
      (set `self.BlueLit` true))
    (:`NewEnumerator5`
      (set `self.RedLit` true)
      (set `self.BlueLit` true))
    (:`NewEnumerator6`
      (set `self.RedLit` true)
      (set `self.GreenLit` true)
      (set `self.BlueLit` true))))

(fn `UserConstructionScript`)