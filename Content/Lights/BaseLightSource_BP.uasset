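; Base Blueprint for a light source actor that holds a colour, chosen by enum, and a cached world transform.
; Construction Script and BeginPlay both force the enum to Red, resolve it through GetColourFromENUM, and store the root's location, rotation and scale.
; SetNewLightColour updates the enum and returns the resolved colour without writing the Colour variable.
; No light component is driven here.
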(event `self.ReceiveBeginPlay`
  (bind _defaultsceneroot (`self.DefaultSceneRoot`))
  (bind _output_get (set `self.Colour_ENUM` "NewEnumerator0"))
  (bind _newparam (`self.GetColourFromENUM` _output_get))
  (set `self.Colour` _newparam)
  (set `self.Location` (`SceneComponent.K2_GetComponentLocation` _defaultsceneroot))
  (set `self.Rotation` (`SceneComponent.K2_GetComponentRotation` _defaultsceneroot))
  (set `self.Scale` (`SceneComponent.K2_GetComponentScale` _defaultsceneroot)))

(fn `GetColourFromENUM`
  (params (ColourENUM :type "/Game/Enums/Colours8_ENUM Enum" :default "NewEnumerator0"))
  (returns (NewParam :type "LinearColor Structure"))
  (switch `/Game/Enums/Colours8_ENUM` ColourENUM
    (:`NewEnumerator0`
      (set `self.Colour` (struct :`R` 1.0 :`A` 1.0)))
    (:`NewEnumerator3`
      (set `self.Colour` (struct :`R` 1.0 :`G` 1.0 :`A` 1.0)))
    (:`NewEnumerator1`
      (set `self.Colour` (struct :`G` 1.0 :`A` 1.0)))
    (:`NewEnumerator4`
      (set `self.Colour` (struct :`G` 1.0 :`B` 1.0 :`A` 1.0)))
    (:`NewEnumerator2`
      (set `self.Colour` (struct :`B` 1.0 :`A` 1.0)))
    (:`NewEnumerator5`
      (set `self.Colour` (struct :`R` 1.0 :`B` 1.0 :`A` 1.0)))
    (:`NewEnumerator6`
      (set `self.Colour` (struct :`R` 1.0 :`G` 1.0 :`B` 1.0 :`A` 1.0)))
    (:`NewEnumerator7`
      (set `self.Colour` (struct :`A` 1.0))))
  (return (`self.Colour`)))

(fn `SetNewLightColour`
  (params (Colour :type "/Game/Enums/Colours8_ENUM Enum" :default "NewEnumerator0"))
  (returns (NewColour :type "LinearColor Structure"))
  (bind _output_get (set `self.Colour_ENUM` Colour))
  (bind _newparam (`self.GetColourFromENUM` _output_get))
  (return _newparam))

(fn `UserConstructionScript`
  (bind _defaultsceneroot (`self.DefaultSceneRoot`))
  (bind _output_get (set `self.Colour_ENUM` "NewEnumerator0"))
  (bind _newparam (`self.GetColourFromENUM` _output_get))
  (set `self.Colour` _newparam)
  (set `self.Location` (`SceneComponent.K2_GetComponentLocation` _defaultsceneroot))
  (set `self.Rotation` (`SceneComponent.K2_GetComponentRotation` _defaultsceneroot))
  (set `self.Scale` (`SceneComponent.K2_GetComponentScale` _defaultsceneroot)))