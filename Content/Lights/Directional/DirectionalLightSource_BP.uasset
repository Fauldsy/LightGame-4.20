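; Directional light variant of a parent light-source Blueprint, with an intensity and a switchable colour.
; The construction script tags its LightType with the first enum entry, and BeginPlay applies the Intensity variable to the DirectionalLight component.
; The SetNewLightColour override gets the colour for an enum value from the parent, applies it to the component, prints the enum name and returns the colour.
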(event `self.ReceiveBeginPlay`
  (`parent.ReceiveBeginPlay`)
  (`LightComponent.SetIntensity` (`self.DirectionalLight`) (`self.Intensity`)))

(fn `SetNewLightColour`
  (params (Colour :type "/Game/Enums/Colours8_ENUM Enum" :default "NewEnumerator0"))
  (returns (NewColour :type "LinearColor Structure"))
  (bind _newcolour (`parent.SetNewLightColour` Colour))
  (`LightComponent.SetLightColor` (`self.DirectionalLight`) _newcolour true)
  (`KismetSystemLibrary.PrintString` (`|GetEnumeratorNameAsString` Colour))
  (return _newcolour))

(fn `UserConstructionScript`
  (`parent.UserConstructionScript`)
  (set `self.LightType` "NewEnumerator0"))