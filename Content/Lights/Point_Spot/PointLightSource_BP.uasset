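; Point light Blueprint that exposes shape and colour settings for placing lights in a level.
; Its construction script calls the parent's, sets a fixed light type, then pushes attenuation radius, source radius, soft source radius and source length onto the PointLight component.
; A colour enum is converted through GetColourFromENUM, stored and applied as the sRGB light colour.
; All event graph nodes are disabled, so it adds no runtime logic.
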(fn `UserConstructionScript`
  (bind _pointlight (`self.PointLight`))
  (`parent.UserConstructionScript`)
  (set `self.LightType` "NewEnumerator1")
  (`PointLightComponent.SetAttenuationRadius` _pointlight (`self.AttenuationRadius`))
  (`PointLightComponent.SetSourceRadius` _pointlight (`self.SourceRadius`))
  (`PointLightComponent.SetSoftSourceRadius` _pointlight (`self.SoftSourceRadius`))
  (`PointLightComponent.SetSourceLength` _pointlight (`self.SourceLength`))
  (bind _newparam (`self.GetColourFromENUM` (`self.Colour_ENUM`)))
  (bind _output_get (set `self.Colour` _newparam))
  (`LightComponent.SetLightColor` (`self.PointLight`) _output_get true))