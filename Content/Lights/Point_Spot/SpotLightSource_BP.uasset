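; A spot light source Blueprint, derived from a parent light class, that configures its TestLight component from exposed properties.
; The construction script sets the light type, resolves a colour enum into Colour, and applies it with attenuation, source shape and cone angle settings.
; SetNewLightColour extends the parent function, pushing the returned colour to the light and passing it back to the caller.
; The event graph has no active logic.
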(fn `SetNewLightColour`
  (params (Colour :type "/Game/Enums/Colours8_ENUM Enum" :default "NewEnumerator0"))
  (returns (NewColour :type "LinearColor Structure"))
  (bind _newcolour (`parent.SetNewLightColour` Colour))
  (`LightComponent.SetLightColor` (`self.TestLight`) _newcolour true)
  (return _newcolour))

(fn `UserConstructionScript`
  (bind _testlight (`self.TestLight`))
  (`parent.UserConstructionScript`)
  (set `self.LightType` "NewEnumerator2")
  (bind _newparam (`self.GetColourFromENUM` (`self.Colour_ENUM`)))
  (set `self.Colour` _newparam)
  (`LightComponent.SetLightColor` (`self.TestLight`) _newparam true)
  (`PointLightComponent.SetAttenuationRadius` _testlight (`self.AttenuationRadius`))
  (`PointLightComponent.SetSourceRadius` _testlight (`self.SourceRadius`))
  (`PointLightComponent.SetSoftSourceRadius` _testlight (`self.SoftSourceRadius`))
  (`PointLightComponent.SetSourceLength` _testlight (`self.SourceLength`))
  (`SpotLightComponent.SetOuterConeAngle` _testlight (`self.OuterConeAngle`))
  (`SpotLightComponent.SetInnerConeAngle` _testlight (`self.InnerConeAngle`)))